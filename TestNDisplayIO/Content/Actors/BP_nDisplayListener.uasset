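; Actor that listens for nDisplay cluster events and prints a debug message for each one it receives.
; It registers itself as a cluster event listener through the API on BeginPlay and removes itself on EndPlay.
; JSON events report their name and type, while binary events report their event ID, with no further handling.
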(event `self.ReceiveBeginPlay`
  ;[1 1 1] Init listener
  (`DisplayClusterBlueprintAPI.AddClusterEventListener` (`DisplayClusterBlueprintLib.GetAPI`) self)
  (`KismetSystemLibrary.PrintString` "Cluster events custom listener started"))

(event `self.ReceiveEndPlay`
  (params (EndPlayReason :type "EEndPlayReason Enum" :default "Destroyed"))
  ;[1 1 1] Init listener
  (`DisplayClusterBlueprintAPI.RemoveClusterEventListener` (`DisplayClusterBlueprintLib.GetAPI`) self))

(event `self.OnClusterEventJson`
  (params (Event :type "DisplayClusterClusterEventJson Structure (by ref)"))
  (bind (_name _type) (break `DisplayClusterClusterEventJson` Event))
  ;[1 1 1] JSON event listener
  (`KismetSystemLibrary.PrintString` (`KismetTextLibrary.Conv_TextToString` (`|FormatText` "Received command {0} of type {1}" _name _type))))

(event `self.OnClusterEventBinary`
  (params (Event :type "DisplayClusterClusterEventBinary Structure (by ref)"))
  ;[1 1 1] BINARY event listener
  (`KismetSystemLibrary.PrintString` (`KismetTextLibrary.Conv_TextToString` (`|FormatText` "Received command with ID {0}" (`.EventId` (break `DisplayClusterClusterEventBinary` Event))))))

(fn `UserConstructionScript`)